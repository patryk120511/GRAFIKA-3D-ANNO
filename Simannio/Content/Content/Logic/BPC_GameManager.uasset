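; BPC_GameManager runs the economy of a building game, tracking money and goods stored in GI_GameInstance.
; Looping timers deduct every building's maintenance, looked up through the controller's building manager, and auto-sell surplus fish, wood and boards above a fixed stock.
; Helper functions add goods, consume materials when stock suffices, and read building output.
; Only fish sales earn money: wood and board payouts multiply by zero, and price lookup reads only the FishP row.
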(event `self.ReceiveBeginPlay`
  (`KismetSystemLibrary.K2_SetTimerDelegate` (delegate `DecrementMoneyByMaintanceCost`) 5.0 true)
  (`KismetSystemLibrary.K2_SetTimer` null "sellProductsAboveCount" 2.0 true))

(event `DecrementMoneyByMaintanceCost`
  (bind _outactors (`GameplayStatics.GetAllActorsOfClass` "/Game/Content/Buildings/BP_BuildingBase.BP_BuildingBase_C"))
  (for _array_element _outactors
    (bind _name (message `/Game/Content/Interfaces/BPI_Interactable.getEnumName` _array_element))
    (bind _cost (`self.getBuildingMaintanceCost` _name))
    (`self.decrementMoney` _cost)))

(event `self.ReceiveTick`
  (params (DeltaSeconds :type "Float (single-precision)")))

(fn `addGoodie`
  (params (product :type "/Game/Content/Logic/Enums/E_Products Enum" :default "NewEnumerator0") (count :type "Float (double-precision)"))
  (bind _asgi_game_instance (cast `/Game/Content/Logic/GI_GameInstance` (`GameplayStatics.GetGameInstance`)))
  (switch `/Game/Content/Logic/Enums/E_Products` product
    (:`NewEnumerator0`
      (set `/Game/Content/Logic/GI_GameInstance.FishCount` (+ (`/Game/Content/Logic/GI_GameInstance.FishCount` _asgi_game_instance) count) _asgi_game_instance))
    (:`NewEnumerator1`
      (set `/Game/Content/Logic/GI_GameInstance.ClothesCount` (+ (`/Game/Content/Logic/GI_GameInstance.ClothesCount` _asgi_game_instance) count) _asgi_game_instance))
    (:`NewEnumerator2`
      (set `/Game/Content/Logic/GI_GameInstance.BoardCount` (+ (`/Game/Content/Logic/GI_GameInstance.BoardCount` _asgi_game_instance) count) _asgi_game_instance))
    (:`NewEnumerator5`
      (set `/Game/Content/Logic/GI_GameInstance.WoodCount` (+ (`/Game/Content/Logic/GI_GameInstance.WoodCount` _asgi_game_instance) count) _asgi_game_instance))
    (:`NewEnumerator4`
      (set `/Game/Content/Logic/GI_GameInstance.WoolCount` (+ (`/Game/Content/Logic/GI_GameInstance.WoolCount` _asgi_game_instance) count) _asgi_game_instance))))

(fn `addProductCountByEnum`)

(fn `decrementMoney`
  (params (value :type "Float (double-precision)"))
  (bind _asgi_game_instance (cast `/Game/Content/Logic/GI_GameInstance` (`GameplayStatics.GetGameInstance`)))
  (set `/Game/Content/Logic/GI_GameInstance.Money` (- (`/Game/Content/Logic/GI_GameInstance.Money` _asgi_game_instance) value) _asgi_game_instance))

(fn `getBuildingMaintanceCost`
  (params (building :type "/Game/Content/Logic/Enums/E_Buildings Enum" :default "NewEnumerator0"))
  (returns (cost :type "Float (double-precision)"))
  (bind _asbp_top_down_controller (cast `/Game/TopDown/Blueprints/BP_TopDownController` (`GameplayStatics.GetPlayerController` 0)))
  (bind (_description _productioncost _productiontime _constructionmaterial _constructionmaterialcount _peopletomaintance _costtomaintance) (`/Game/Content/Logic/BP_BuildingManager.getBuildingInfoFromTable` (`/Game/TopDown/Blueprints/BP_TopDownController.BP_BuildingManager` _asbp_top_down_controller) building))
  (return _costtomaintance))

(fn `getBuildingProductGoodieAndCount`
  (params (building :type "/Game/Content/Logic/Enums/E_Buildings Enum" :default "NewEnumerator0"))
  (returns (product :type "/Game/Content/Logic/Enums/E_Products Enum") (count :type "Float (double-precision)"))
  (bind _asbp_top_down_controller (cast `/Game/TopDown/Blueprints/BP_TopDownController` (`GameplayStatics.GetPlayerController` 0)))
  (bind (_description _productioncost _productiontime _constructionmaterial _constructionmaterialcount _peopletomaintance _costtomaintance _productoutput _productoutputcount) (`/Game/Content/Logic/BP_BuildingManager.getBuildingInfoFromTable` (`/Game/TopDown/Blueprints/BP_TopDownController.BP_BuildingManager` _asbp_top_down_controller) building))
  (return _productoutput _productoutputcount))

(fn `getProductValue`
  (params (product :type "/Game/Content/Logic/Enums/E_Products Enum" :default "NewEnumerator0"))
  (returns (value :type "Float (double-precision)"))
  (bind _returnvalue (`|GetDataTableRow` "/Game/Content/Logic/Data/DT_Products.DT_Products" "FishP")
    (:`then`
      (bind (_product _value) (break `/Game/Content/Logic/Data/DS_Products` _returnvalue))
      (if (`|EnumEquality` product _product)
        (return _value)))))

(fn `incrementMoney`
  (params (value :type "Float (double-precision)"))
  (bind _asgi_game_instance (cast `/Game/Content/Logic/GI_GameInstance` (`GameplayStatics.GetGameInstance`)))
  (set `/Game/Content/Logic/GI_GameInstance.Money` (+ (`/Game/Content/Logic/GI_GameInstance.Money` _asgi_game_instance) value) _asgi_game_instance))

(fn `sellProductsAboveCount`
  (locals (temp :type "Float (double-precision)"))
  (bind _asgi_game_instance (cast `/Game/Content/Logic/GI_GameInstance` (`GameplayStatics.GetGameInstance`)))
  (bind _fishcount (`/Game/Content/Logic/GI_GameInstance.FishCount` _asgi_game_instance))
  (if (> _fishcount 25.0)
    (bind _returnvalue (* (- _fishcount 25.0) -1.0))
    (set `local.temp` _returnvalue)
    (`self.addGoodie` "NewEnumerator0" _returnvalue)
    (bind _value (`self.getProductValue` "NewEnumerator0"))
    (bind _returnvalue_2 (* _value (* (`local.temp`) -1.0)))
    (`KismetSystemLibrary.PrintString` (`KismetStringLibrary.Conv_DoubleToString` _returnvalue_2))
    (`self.incrementMoney` _returnvalue_2))
  (bind _woodcount (`/Game/Content/Logic/GI_GameInstance.WoodCount` _asgi_game_instance))
  (if (> _woodcount 25.0)
    (set `local.temp` 0.0)
    (`self.addGoodie` "NewEnumerator5" (* (- _woodcount 25.0) -1.0))
    (bind _value_2 (`self.getProductValue` "NewEnumerator5"))
    (`self.incrementMoney` (* (* (`local.temp`) -1.0) _value_2)))
  (bind _boardcount (`/Game/Content/Logic/GI_GameInstance.BoardCount` _asgi_game_instance))
  (if (> _boardcount 25.0)
    (set `local.temp` 0.0)
    (`self.addGoodie` "NewEnumerator2" (* (- _boardcount 25.0) -1.0))
    (bind _value_3 (`self.getProductValue` "NewEnumerator2"))
    (`self.incrementMoney` (* (* (`local.temp`) -1.0) _value_3))))

(fn `useMaterial`
  (params (material :type "/Game/Content/Logic/Enums/E_Materials Enum" :default "NewEnumerator1") (count :type "Float (double-precision)"))
  (returns (value :type Boolean))
  (bind _asgi_game_instance (cast `/Game/Content/Logic/GI_GameInstance` (`GameplayStatics.GetGameInstance`)))
  (switch `/Game/Content/Logic/Enums/E_Materials` material
    (:`NewEnumerator1`
      (bind _returnvalue (- (`/Game/Content/Logic/GI_GameInstance.WoodCount` _asgi_game_instance) count))
      (if (>= _returnvalue 0.0)
        (set `/Game/Content/Logic/GI_GameInstance.WoodCount` _returnvalue _asgi_game_instance)
        (return true)
        (else
          (return false))))
    (:`NewEnumerator0`
      (bind _returnvalue_2 (- (`/Game/Content/Logic/GI_GameInstance.WoolCount` _asgi_game_instance) count))
      (if (>= _returnvalue_2 0.0)
        (set `/Game/Content/Logic/GI_GameInstance.WoolCount` _returnvalue_2 _asgi_game_instance)
        (return true)
        (else
          (return false))))
    (:`NewEnumerator4`
      (bind _returnvalue_3 (- (`/Game/Content/Logic/GI_GameInstance.BoardCount` _asgi_game_instance) count))
      (if (>= _returnvalue_3 0.0)
        (set `/Game/Content/Logic/GI_GameInstance.BoardCount` _returnvalue_3 _asgi_game_instance)
        (return true)
        (else
          (return false))))))