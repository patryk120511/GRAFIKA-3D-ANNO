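; BP_BuildingManager tracks which map locations are occupied by buildings and supplies building type data.
; The PlacesOnMap map links locations to buildings, with functions to add, look up, check and remove entries by location or actor.
; Building info comes from DT_Buildings for Fish and Wood factories only, and an if-chain converts classes to types, defaulting to House.
; Placement and preview functions are empty stubs that only check validity.
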(event `self.ReceiveBeginPlay`
  (bind _asbp_game_state (cast `/Game/Content/Logic/BP_GameState` (`GameplayStatics.GetGameMode`)))
  (set `self.gameState` _asbp_game_state))

(fn `addObjectToLocation`
  (params (Location :type "Vector2D Structure") (Object :type "Actor Object Reference"))
  (`BlueprintMapLibrary.Map_Add` (`self.PlacesOnMap`) Location Object))

(fn `AddTakenPlace`
  (params (NewVec :type "Vector2D Structure") (Building :type "Actor Object Reference"))
  (`BlueprintMapLibrary.Map_Add` (`self.PlacesOnMap`) NewVec Building))

(fn `CheckIfPlaceCanBeTaken`
  (params (ValueToCheck :type "Vector2D Structure"))
  (returns (NewParam :type Boolean))
  (bind _keypin (`|MapForEach` (`self.PlacesOnMap`))
    (:`then`
      (if (`KismetMathLibrary.EqualExactly_Vector2DVector2D` _keypin ValueToCheck)
        (return false)))
    (:`CompletedPin`
      (return true))))

(fn `getBuildingByClass`
  (params (Class :type "Actor Class Reference"))
  (returns (Building :type "/Game/Content/Logic/Enums/E_Buildings Enum"))
  (if (== Class "/Game/Content/Buildings/BP_Home.BP_Home_C")
    (return "NewEnumerator0")
    (elif (== Class "/Game/Content/Buildings/BP_FishFactory.BP_FishFactory_C")
      (return "NewEnumerator1")
      (elif (== Class "/Game/Content/Buildings/BP_WoodFactory.BP_WoodFactory_C")
        (return "NewEnumerator2")
        (elif (== Class "/Game/Content/Buildings/BP_BoardFactory.BP_BoardFactory_C")
          (return "NewEnumerator3")
          (elif (== Class "/Game/Content/Buildings/BP_Home.BP_Home_C")
            (return "NewEnumerator0")
            (elif (== Class "/Game/Content/Buildings/BP_Home.BP_Home_C")
              (return "NewEnumerator0")
              (else
                (if (== Class "/Game/Content/Buildings/BP_Home.BP_Home_C")
                  _
                  (else
                    _))
                (return "NewEnumerator0")))))))))

(fn `getBuildingInfoFromTable`
  (params (Building :type "/Game/Content/Logic/Enums/E_Buildings Enum" :default "NewEnumerator0"))
  (returns (Description :type String) (ProductionCost :type "Float (double-precision)") (ProductionTime :type "Float (double-precision)") (ConstructionMaterial :type "/Game/Content/Logic/Enums/E_Materials Enum") (ConstructionMaterialCount :type "Float (double-precision)") (PeopleToMaintance :type Integer) (CostToMaintance :type "Float (double-precision)") (ProductOutput :type "/Game/Content/Logic/Enums/E_Products Enum") (ProductOutputCount :type "Float (double-precision)") (OutputTime :type "Float (double-precision)"))
  (switch `/Game/Content/Logic/Enums/E_Buildings` Building
    (:`NewEnumerator1`
      (bind _returnvalue (`|GetDataTableRow` "/Game/Content/Logic/Data/DT_Buildings.DT_Buildings" "FishF")
        (:`then`
          (bind (_key _value) (`BlueprintMapLibrary.Map_GetKeyValueByIndex` (`.ConstructionCost_28_C6C898CA44A6FA82C135D5B67571BF6F` (break `/Game/Content/Logic/Data/DS_Buildings` _returnvalue))))
          (bind (_key_2 _value_2) (`BlueprintMapLibrary.Map_GetKeyValueByIndex` (`.ProductsOutput_36_5B1251894E660B8E92132AA14BA85A96` (break `/Game/Content/Logic/Data/DS_Buildings` _returnvalue))))
          (return (`.Description_15_F8DC65C24D528E633F6C938424F1A578` (break `/Game/Content/Logic/Data/DS_Buildings` _returnvalue)) (`.ProductionCost_10_FC1A650248A32B3BED6643A738339223` (break `/Game/Content/Logic/Data/DS_Buildings` _returnvalue)) (`.ProductionTime_11_F9D82CBE425607900FBECBB62CD82F69` (break `/Game/Content/Logic/Data/DS_Buildings` _returnvalue)) _key _value (`.PeopleToMaintance_24_00F1B4B041A50D9CF92B308C1DC96B9F` (break `/Game/Content/Logic/Data/DS_Buildings` _returnvalue)) (`.CostToMaintance_27_6F7BACD54A5C5C3190A4F896E3F5060C` (break `/Game/Content/Logic/Data/DS_Buildings` _returnvalue)) _key_2 _value_2 (`.ProductsOutputTime_40_2C5ED20D40A4E3B83F24FAAB01DEFCA5` (break `/Game/Content/Logic/Data/DS_Buildings` _returnvalue))))))
    (:`NewEnumerator2`
      (bind _returnvalue_2 (`|GetDataTableRow` "/Game/Content/Logic/Data/DT_Buildings.DT_Buildings" "WoodF")
        (:`then`
          (bind (_key_3 _value_3) (`BlueprintMapLibrary.Map_GetKeyValueByIndex` (`.ConstructionCost_28_C6C898CA44A6FA82C135D5B67571BF6F` (break `/Game/Content/Logic/Data/DS_Buildings` _returnvalue_2))))
          (bind (_key_4 _value_4) (`BlueprintMapLibrary.Map_GetKeyValueByIndex` (`.ProductsOutput_36_5B1251894E660B8E92132AA14BA85A96` (break `/Game/Content/Logic/Data/DS_Buildings` _returnvalue_2))))
          (return (`.Description_15_F8DC65C24D528E633F6C938424F1A578` (break `/Game/Content/Logic/Data/DS_Buildings` _returnvalue_2)) (`.ProductionCost_10_FC1A650248A32B3BED6643A738339223` (break `/Game/Content/Logic/Data/DS_Buildings` _returnvalue_2)) (`.ProductionTime_11_F9D82CBE425607900FBECBB62CD82F69` (break `/Game/Content/Logic/Data/DS_Buildings` _returnvalue_2)) _key_3 _value_3 (`.PeopleToMaintance_24_00F1B4B041A50D9CF92B308C1DC96B9F` (break `/Game/Content/Logic/Data/DS_Buildings` _returnvalue_2)) (`.CostToMaintance_27_6F7BACD54A5C5C3190A4F896E3F5060C` (break `/Game/Content/Logic/Data/DS_Buildings` _returnvalue_2)) _key_4 _value_4 (`.ProductsOutputTime_40_2C5ED20D40A4E3B83F24FAAB01DEFCA5` (break `/Game/Content/Logic/Data/DS_Buildings` _returnvalue_2))))))))

(fn `getObjectByLocation`
  (params (NewParam :type "Vector2D Structure"))
  (returns (NewParam1 :type "Actor Object Reference"))
  (bind (_value _returnvalue) (`BlueprintMapLibrary.Map_Find` (`self.PlacesOnMap`) NewParam))
  (if _returnvalue
    (return _value)
    (else
      (return null))))

(fn `removeTakenPlace`
  (params (placeToRemove :type "Vector2D Structure"))
  (`BlueprintMapLibrary.Map_Remove` (`self.PlacesOnMap`) placeToRemove))

(fn `removeTakenPlaceByActor`
  (params (actor :type "Actor Object Reference"))
  (bind _placesonmap (`self.PlacesOnMap`))
  (bind (_keypin _valuepin) (`|MapForEach` _placesonmap)
    (:`then`
      (if (== _valuepin actor)
        (`BlueprintMapLibrary.Map_Remove` _placesonmap _keypin)))))

(fn `tryPlaceBuilding`
  (bind _asbp_game_state (cast `/Game/Content/Logic/BP_GameState` (`GameplayStatics.GetGameMode`)))
  (`/Game/Content/Logic/BP_GameState.selectionMode` _asbp_game_state
    (:`then`)
    (:`else`)))

(fn `trySpawnObjectPreview`
  (`/Game/Content/Logic/BP_GameState.selectionMode` (`self.gameState`)
    (:`then`
      (`self.selectedBuildingPrev`
        (:`then`)
        (:`else`)))
    (:`else`)))