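; BP_WordGenerator is an early procedural world generator that builds a flat grid of points and a mesh section on BeginPlay.
; SetVerticies loops over WorldX and WorldY, adding Scale-spaced vertices at a fixed height and marking each with a debug sphere.
; Triangle indices are placeholders: the loop adds a unique zero and SetTriangles appends one hardcoded triangle, so the grid is not triangulated.
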(event `self.ReceiveBeginPlay`
  (`self.setVerticies`)
  (`self.setTriangles`)
  (`ProceduralMeshComponent.CreateMeshSection_LinearColor` :`self` (`self.ProceduralMesh`) :`Vertices` (`self.Verticies`) :`Triangles` (`self.Triangles`)))

(fn `setTriangles`
  (`KismetArrayLibrary.Array_Add` (`self.Triangles`))
  (`KismetArrayLibrary.Array_Add` (`self.Triangles`) 1)
  (`KismetArrayLibrary.Array_Add` (`self.Triangles`) 2))

(fn `setVerticies`
  (locals (X :type Integer) (Y :type Integer))
  (bind _returnvalue (`KismetMathLibrary.MakeVector` (`KismetMathLibrary.Conv_IntToDouble` (* (`local.X`) (`self.scale`))) (`KismetMathLibrary.Conv_IntToDouble` (* (`local.Y`) (`self.scale`))) 100.0))
  (for _index (range (+ (`self.WorldX`) 1))
    (set `local.X` _index)
    (for _index_2 (range (+ (`self.WorldY`) 1))
      (set `local.Y` _index_2)
      (`KismetArrayLibrary.Array_AddUnique` (`self.Verticies`) _returnvalue)
      (`KismetSystemLibrary.DrawDebugSphere` _returnvalue 10.0 12 (struct :`G` 0.022549 :`B` 1.0 :`A` 1.0) 200.0)
      (`KismetArrayLibrary.Array_AddUnique` (`self.Triangles`)))))

(fn `UserConstructionScript`)