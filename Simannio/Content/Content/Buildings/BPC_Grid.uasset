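; BPC_Grid is a Blueprint component in the Buildings folder that snaps world locations to a square grid.
; SnapToGrid rounds X and Y to the nearest multiple of GridSize, then adds half a cell to each and returns Z as zero.
; Because it rounds rather than floors before the offset, the result is not always the center of the cell containing the input.
; The event graph holds only disabled placeholder events.
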(fn `SnapToGrid`
  (params (Location :type "Vector Structure"))
  (returns (NewParam :type "Vector Structure"))
  (bind _gridsize (`self.GridSize`))
  (bind _returnvalue (/ _gridsize 2.0))
  (return (`KismetMathLibrary.MakeVector` (+ (* (`KismetMathLibrary.Round` (/ Location_X _gridsize)) _gridsize) _returnvalue) (+ (* (`KismetMathLibrary.Round` (/ Location_Y _gridsize)) _gridsize) _returnvalue))))