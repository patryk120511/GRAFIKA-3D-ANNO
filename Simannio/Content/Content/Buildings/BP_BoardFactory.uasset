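; Board factory building actor that periodically produces goods, described in its Polish info text as turning wood into planks.
; A looping timer started on BeginPlay asks the game manager component on BP_TopDownGameMode for this building type's product and count, then adds them through AddGoodie.
; Getters expose the info text, building enum value and actor reference.
; No wood consumption happens in this Blueprint.
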(event `self.ReceiveBeginPlay`
  (`KismetSystemLibrary.K2_SetTimerDelegate` (delegate `/Game/Content/Interfaces/BPI_GameManagment.produceGoodie`) 7.0 true))

(event `/Game/Content/Interfaces/BPI_GameManagment.produceGoodie`
  (bind _asbp_top_down_game_mode (cast `/Game/TopDown/Blueprints/BP_TopDownGameMode` (`GameplayStatics.GetGameMode`)))
  (bind (_product _count) (`/Game/Content/Logic/BPC_GameManager.getBuildingProductGoodieAndCount` (`/Game/TopDown/Blueprints/BP_TopDownGameMode.BPC_GameManager` _asbp_top_down_game_mode) "NewEnumerator3"))
  (`/Game/Content/Logic/BPC_GameManager.addGoodie` (`/Game/TopDown/Blueprints/BP_TopDownGameMode.BPC_GameManager` _asbp_top_down_game_mode) _product _count))

(fn `getActor`
  (returns (actor :type "Actor Object Reference"))
  (return self))

(fn `getEnumName`
  (returns (name :type "/Game/Content/Logic/Enums/E_Buildings Enum"))
  (return "NewEnumerator3"))

(fn `getInfo`
  (returns (info :type String))
  (return "Zmieniamy drzewo na deski"))

(fn `UserConstructionScript`)