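; BP_FishFactory is a fish factory building that periodically produces goods for the game.
; A looping timer started on BeginPlay looks up product and count for its building enum through the GameManager component on BP_TopDownGameMode, then adds them there.
; Simple getters expose its building type, actor reference and a Polish description ("Łowimy ryby", we catch fish).
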(event `self.ReceiveBeginPlay`
  (`KismetSystemLibrary.K2_SetTimerDelegate` (delegate `/Game/Content/Interfaces/BPI_GameManagment.produceGoodie`) 5.0 true))

(event `/Game/Content/Interfaces/BPI_GameManagment.produceGoodie`
  (bind _name (`/Game/Content/Interfaces/BPI_Interactable.getEnumName`))
  (bind _asbp_top_down_game_mode (cast `/Game/TopDown/Blueprints/BP_TopDownGameMode` (`GameplayStatics.GetGameMode`)))
  (bind (_product _count) (`/Game/Content/Logic/BPC_GameManager.getBuildingProductGoodieAndCount` (`/Game/TopDown/Blueprints/BP_TopDownGameMode.BPC_GameManager` _asbp_top_down_game_mode) _name))
  (`/Game/Content/Logic/BPC_GameManager.addGoodie` (`/Game/TopDown/Blueprints/BP_TopDownGameMode.BPC_GameManager` _asbp_top_down_game_mode) _product _count))

(fn `getActor`
  (returns (actor :type "Actor Object Reference"))
  (return self))

(fn `getEnumName`
  (returns (name :type "/Game/Content/Logic/Enums/E_Buildings Enum"))
  (return "NewEnumerator1"))

(fn `getInfo`
  (returns (info :type String))
  (return "Łowimy ryby"))

(fn `UserConstructionScript`)